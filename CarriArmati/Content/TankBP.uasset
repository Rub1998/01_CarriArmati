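; Player tank pawn Blueprint that wires movement, camera and firing input to its components.
; BeginPlay hands the aiming component to the TankPlayerController, gives it the barrel and turret, and initializes the movement component with both tracks.
; Axis inputs drive each track directly or send forward and lateral intents to the movement component.
; Azimuth and elevation inputs rotate the scene and spring arm separately, while Spara fires through the aiming component.
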(event `self.ReceiveBeginPlay`
  (bind _aimingcpp (`self.AimingCPP`))
  (`TankControllerCPP.SetAim` (cast `/Game/TankPlayerController` (`GameplayStatics.GetPlayerController` 0) :!pure true) _aimingcpp)
  (`AimingCPP.SetCannone` _aimingcpp (`self.Barrel`))
  (`AimingCPP.SetTorre` _aimingcpp (`self.Turret`))
  (`Movimento.Initialize` (`self.Movimento`) (`self.TrackDX`) (`self.TrackSX`)))

(event `InputAxis|CingoloSR`
  (params (AxisValue :type "Float (single-precision)"))
  (`MeshCingolo.RichiestaMovimento` (`self.TrackDX`) AxisValue))

(event `InputAxis|Levatura`
  (params (AxisValue :type "Float (single-precision)"))
  (`SceneComponent.K2_AddLocalRotation` (`self.SpringArm`) (`KismetMathLibrary.MakeRotator` 0.0 AxisValue) false false))

(event `InputAxis|CingoloSF`
  (params (AxisValue :type "Float (single-precision)"))
  (`MeshCingolo.RichiestaMovimento` (`self.TrackSX`) AxisValue))

(event `InputAxis|Azimuth`
  (params (AxisValue :type "Float (single-precision)"))
  (`SceneComponent.K2_AddLocalRotation` (`self.Scene`) (`KismetMathLibrary.MakeRotator` 0.0 0.0 AxisValue) false false))

(event `InputAction|Spara`
  (params (Key :type "Key Structure"))
  (:`Pressed`
    (`AimingCPP.SparaReal` (`self.AimingCPP`))))

(event `InputAxis|MoveForward`
  (params (AxisValue :type "Float (single-precision)"))
  (`Movimento.IntenzioneAvanti` (`self.Movimento`) AxisValue))

(event `InputAxis|MoveRight`
  (params (AxisValue :type "Float (single-precision)"))
  (`Movimento.IntenzioneLaterale` (`self.Movimento`) AxisValue))

(fn `UserConstructionScript`)